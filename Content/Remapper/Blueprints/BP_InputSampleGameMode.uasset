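; Sample GameMode that hosts a pause-time input remapping menu and takes player input directly.
; The Pause action shows the remapper widget with mouse and gamepad cursors, and Resume reverses this.
; In bind mode, any key press rewrites the selected action mapping, substituting the bottom face button for mouse clicks during gamepad binding.
; Tick prints current bindings on screen, and Escape quits outside bind mode.
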(event Custom|Resume
  ;[1 1 1] Pause解除 マウスカーソルを非表示にし、ConfigのUIを非表示にする
  (Widget|RemovefromParent (Variables|Default|GetInputWidgetRef))
  (Variables|/Script/Engine.PlayerController|SetbShowMouseCursor (Game|GetPlayerController 0) false)
  (Game|SetGamePaused false)
  (Class|PSGamepadFunctionLibrary|DisableGamepadCursor))

(event EventBeginPlay
  ;[1 1 1] Widgetの作成とGameMode内でのInput有効化
  (bind _returnvalue (UserInterface|CreateWidget "/Game/Remapper/UserInterface/WBP_InputRemmapper.WBP_InputRemmapper_C"))
  (Variables|Default|SetInputWidgetRef _returnvalue)
  (Input|EnableInput (Game|GetPlayerController 0)))

(event EventTick
  (params (DeltaSeconds :type Float%20%28single-precision%29))
  ;[1 0.25 0.25] 割り当てられているKey一覧のLogを表示
  (for _array_element (Class|PSInputFunctionLibrary|GetAllActionMappingName)
    (Development|PrintString (Utilities|String|Append (.bindname _array_element) " : " (.keyasstring _array_element)) true false "(R=0.000000,G=0.660000,B=1.000000,A=1.000000)" 0.0)))

(event Input|ActionEvents|InputActionPause
  (params (Key :type Key%20Structure :default "None"))
  (bind _inputwidgetref (Variables|Default|GetInputWidgetRef))
  ;[1 1 1] Enter押下時にPauseしてConfigUIとマウスカーソルを表示
  (:Pressed
    (if (not (UserInterface|Viewport|IsinViewport _inputwidgetref))
      (UserInterface|Viewport|AddtoViewport _inputwidgetref 0)
      (Variables|/Script/Engine.PlayerController|SetbShowMouseCursor (Game|GetPlayerController 0) true)
      (Class|PSGamepadFunctionLibrary|EnableGamepadCursor)
      (Game|SetGamePaused true))))

(event Input|KeyboardEvents|AnyKey
  (params (Key :type Key%20Structure :default "None"))
  (bind _inputwidgetref (Variables|Default|GetInputWidgetRef))
  (bind _inputwidgetref_2 (Variables|Default|GetInputWidgetRef))
  (bind _inputtype (Variables|/Game/Remapper/UserInterface/WBP_InputRemmapper.WBP_InputRemmapper_C|GetInputType _inputwidgetref_2))
  (bind _currentbindactionname (Variables|/Game/Remapper/UserInterface/WBP_InputRemmapper.WBP_InputRemmapper_C|GetCurrentBindActionName _inputwidgetref))
  ;[1 1 1] キーの割当
  (:Pressed
    (if (and (UserInterface|Viewport|IsinViewport _inputwidgetref_2) (Variables|/Game/Remapper/UserInterface/WBP_InputRemmapper.WBP_InputRemmapper_C|GetIsBindMode _inputwidgetref_2))
      (if (and (Class|KismetInputLibrary|KeyIsMouseButton Key) (Utilities|Enum|Equal(Enum) _inputtype "Gamepad"))
        (Class|PSInputFunctionLibrary|UpdateActionMapping _currentbindactionname "Gamepad_FaceButton_Bottom" "Gamepad")
        (Default|UpdateKeyText _inputwidgetref _currentbindactionname "Gamepad")
        (else
          (Class|PSInputFunctionLibrary|UpdateActionMapping _currentbindactionname Key _inputtype)
          (Default|UpdateKeyText _inputwidgetref _currentbindactionname _inputtype)))
      (Default|EscapeBindMode (Variables|Default|GetInputWidgetRef)))))

(event Input|KeyboardEvents|Escape
  (params (Key :type Key%20Structure :default "None"))
  ;[1 1 1] Escape押下時にConfigを開いてなければゲーム終了
  (:Pressed
    (if (not (Variables|/Game/Remapper/UserInterface/WBP_InputRemmapper.WBP_InputRemmapper_C|GetIsBindMode (Variables|Default|GetInputWidgetRef)))
      (Game|QuitGame 0 "Quit" false))))

(fn ConstructionScript)