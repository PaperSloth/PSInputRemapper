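; Game mode for an input-remapping sample that lets the player rebind the Jump action at runtime.
; It creates a WBP_InputRemmapper widget, which Enter shows while pausing the game; Resume reverses this.
; In the widget's bind mode, AnyKey updates the Jump mapping and key text, while Enter or Escape cancels.
; Escape otherwise quits, and Tick prints Jump's current bindings for debugging.
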(event Custom|Resume
  ;[1 1 1] Pause解除 マウスカーソルを非表示にし、ConfigのUIを非表示にする
  (Widget|RemovefromParent (Variables|Default|GetInputWidgetRef))
  (Variables|/Script/Engine.PlayerController|SetbShowMouseCursor (Game|GetPlayerController 0) false)
  (Game|SetGamePaused false))

(event EventBeginPlay
  ;[1 1 1] Widgetの作成とGameMode内でのInput有効化
  (bind _returnvalue (UserInterface|CreateWidget "/PSInputRemapper/UserInterface/WBP_InputRemmapper.WBP_InputRemmapper_C"))
  (Variables|Default|SetInputWidgetRef _returnvalue)
  (Input|EnableInput (Game|GetPlayerController 0)))

(event EventTick
  (params (DeltaSeconds :type Float%20%28single-precision%29))
  ;[1 0.25 0.25] Jumpに割り当てられているKey一覧のLogを表示
  (bind _inputarray (Class|PSInputFunctionLibrary|FindCurrentActionMappings (Variables|Default|GetActionNameJump)))
  (for _array_element _inputarray
    (Development|PrintString (Utilities|String|Append (.bindname _array_element) " : " (.keyasstring _array_element)) true true "(R=0.000000,G=0.660000,B=1.000000,A=1.000000)" 0.0)))

(event Input|KeyboardEvents|Enter
  (params (Key :type Key%20Structure))
  (bind _inputwidgetref (Variables|Default|GetInputWidgetRef))
  ;[1 1 1] Enter押下時にPauseしてConfigUIとマウスカーソルを表示
  (:Pressed
    (if (not (UserInterface|Viewport|IsinViewport _inputwidgetref))
      (UserInterface|Viewport|AddtoViewport _inputwidgetref 0)
      (Variables|/Script/Engine.PlayerController|SetbShowMouseCursor (Game|GetPlayerController 0) true)
      (Game|SetGamePaused true))))

(event Input|KeyboardEvents|AnyKey
  (params (Key :type Key%20Structure))
  (bind _inputwidgetref (Variables|Default|GetInputWidgetRef))
  (bind _inputwidgetref_2 (Variables|Default|GetInputWidgetRef))
  (bind _actionnamejump (Variables|Default|GetActionNameJump))
  (bind _inputtype (Variables|/PSInputRemapper/UserInterface/WBP_InputRemmapper.WBP_InputRemmapper_C|GetInputType _inputwidgetref))
  ;[1 1 1] Jumpへのキーの割当(Enter/Escapeは除く)
  (:Pressed
    (if (and (UserInterface|Viewport|IsinViewport _inputwidgetref) (Variables|/PSInputRemapper/UserInterface/WBP_InputRemmapper.WBP_InputRemmapper_C|GetIsBindMode _inputwidgetref))
      (if (or (== Key "Enter") (== Key "Escape"))
        (Default|EscapeBindMode _inputwidgetref_2)
        (else
          (Class|PSInputFunctionLibrary|UpdateActionMapping _actionnamejump Key _inputtype)
          (Default|UpdateKeyText _inputwidgetref_2 _actionnamejump _inputtype))))))

(event Input|KeyboardEvents|Escape
  (params (Key :type Key%20Structure))
  ;[1 1 1] Escape押下時にConfigを開いてなければゲーム終了
  (:Pressed
    (if (not (Variables|/PSInputRemapper/UserInterface/WBP_InputRemmapper.WBP_InputRemmapper_C|GetIsBindMode (Variables|Default|GetInputWidgetRef)))
      (Game|QuitGame 0 "Quit" false))))

(fn ConstructionScript)